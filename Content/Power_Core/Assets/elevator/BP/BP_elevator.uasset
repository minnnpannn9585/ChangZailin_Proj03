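; Elevator actor that moves its Door1 component vertically when something overlaps one of two trigger boxes.
; Box plays a Timeline that drives Door1's relative Z downward, and Box1 reverses it, each with an elevator sound.
; Down and Up flags block a trigger while the opposite move is flagged, and both clear when the Timeline finishes.
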(event `self.Box.OnComponentBeginOverlap`
  (params (OverlappedComponent :type "PrimitiveComponent Object Reference") (OtherActor :type "Actor Object Reference") (OtherComp :type "PrimitiveComponent Object Reference") (OtherBodyIndex :type Integer) (bFromSweep :type Boolean) (SweepResult :type "HitResult Structure (by ref)"))
  (set `self.Down?` true)
  (if (not (`self.up?`))
    (`GameplayStatics.SpawnSoundAtLocation` "/Game/Power_Core/Audio/SW_Elevator.SW_Elevator" (0.0 0.0 0.0) (struct) 0.5 1.0 0.0 null null)
    (bind (_direction _door_1) (`Timeline|Timeline` :!label _label)
      (:`Update`
        (`SceneComponent.K2_SetRelativeLocation` (`self.door_1_`) (`KismetMathLibrary.MakeVector` 0.0 0.0 (* _door_1 -1570.0)) false false))
      (:`Finished`
        (set `self.Down?` false)
        (set `self.up?` false)))))

(event `self.Box1.OnComponentBeginOverlap`
  (params (OverlappedComponent :type "PrimitiveComponent Object Reference") (OtherActor :type "Actor Object Reference") (OtherComp :type "PrimitiveComponent Object Reference") (OtherBodyIndex :type Integer) (bFromSweep :type Boolean) (SweepResult :type "HitResult Structure (by ref)"))
  (set `self.up?` true)
  (if (not (`self.Down?`))
    (`GameplayStatics.SpawnSoundAtLocation` "/Game/Power_Core/Audio/SW_Elevator.SW_Elevator" (0.0 0.0 0.0) (struct) 0.5 1.0 0.0 null null)
    (goto _label :!via `Reverse`)))

(fn `UserConstructionScript`)