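; Sliding door Blueprint that opens when anything begins overlapping its Box trigger and closes itself on a timer.
; After a short delay, the overlap plays an opening sound and a Timeline that slides Door2 along its local Y axis.
; When the Timeline finishes, an IsOpen check gates a hold delay, closing sound and reverse playback, so the closing pass does not retrigger itself.
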(event `self.Box.OnComponentBeginOverlap`
  (params (OverlappedComponent :type "PrimitiveComponent Object Reference") (OtherActor :type "Actor Object Reference") (OtherComp :type "PrimitiveComponent Object Reference") (OtherBodyIndex :type Integer) (bFromSweep :type Boolean) (SweepResult :type "HitResult Structure (by ref)"))
  (`KismetSystemLibrary.Delay` 0.5)
  (set `self.Is_Open` true)
  (`GameplayStatics.SpawnSoundAtLocation` "/Game/Power_Core/Audio/SW_Door_Open_2.SW_Door_Open_2" (0.0 0.0 0.0) (struct) 0.5 1.0 0.0 null null)
  (bind (_direction _door_1) (`Timeline|Timeline` :!label _label)
    (:`Update`
      (`SceneComponent.K2_SetRelativeLocation` (`self.door_2_`) (`KismetMathLibrary.MakeVector` 0.0 (* _door_1 220.0)) false false))
    (:`Finished`
      (if (`self.Is_Open`)
        (`KismetSystemLibrary.Delay` 7.0)
        (`GameplayStatics.SpawnSoundAtLocation` "/Game/Power_Core/Audio/SW_Door_2_Close.SW_Door_2_Close" (0.0 0.0 0.0) (struct) 0.5 1.0 0.0 null null)
        (set `self.Is_Open` false)
        (goto _label :!via `Reverse`)))))

(fn `UserConstructionScript`)